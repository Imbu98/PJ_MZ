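; BP_StartRoom is the starting room actor in the dungeon generator, and it sets up the stage NPC for that room.
; On BeginPlay, after calling its parent logic, it spawns a BP_StageNPC at its Scene component's world transform, adjusting for collisions but always spawning.
; It then passes its SMDoor to the NPC as DoorMeshComp, giving the NPC a reference to the room's door.
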(event `self.ReceiveBeginPlay`
  (`parent.ReceiveBeginPlay`)
  (bind _returnvalue (`|SpawnActorFromClass` "/Game/HT/HT_Charaters/NPC/BP_StageNPC.BP_StageNPC_C" (`SceneComponent.K2_GetComponentToWorld` (`self.Scene`)) "AdjustIfPossibleButAlwaysSpawn" "MultiplyWithRoot" null null))
  (set `StageNPC.DoorMeshComp` (`self.SM_Door`) _returnvalue))

(fn `UserConstructionScript`
  (`parent.UserConstructionScript`))