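; Base actor for photographable objects that plays a dissolve effect with particles and light when its picture is taken.
; Construction creates a dynamic M_Camera material and derives the dissolve distance from half the mesh's local bounds diagonal.
; PictureTaken sets an object-space origin and spawns NS_HitDissolve on the mesh.
; A timeline drives material and Niagara dissolve distance plus point light intensity, then resets the material's distance to zero.
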(event `self.PictureTaken`
  (bind _returnvalue (`self.GetTransform`))
  (bind _material (`self.Material`))
  (bind _returnvalue_2 (`KismetMathLibrary.InverseTransformLocation` _returnvalue (0.0 0.0 0.0)))
  (`MaterialInstanceDynamic.SetVectorParameterValue` (`self.Material`) "Dissolve Origin Object Space" (`KismetMathLibrary.Conv_VectorToLinearColor` _returnvalue_2))
  (bind _returnvalue_3 (`NiagaraFunctionLibrary.SpawnSystemAttached` "/Game/NiagaraExamples/FX_Misc/NS_HitDissolve.NS_HitDissolve" (`self.StaticMeshComp`) "None" (0.0 0.0 0.0) (struct) "SnapToTarget" true true "AutoRelease"))
  (bind _output_get (set `self.Niagara System` _returnvalue_3))
  (`NiagaraComponent.SetVariablePosition` _output_get "Dissolve Origin" _returnvalue_2)
  (`NiagaraComponent.SetVariableVec3` _output_get "Burst Direction" (`KismetMathLibrary.InverseTransformDirection` _returnvalue (0.0 0.0 0.0)))
  (bind (_direction _dissolve _light_intensity) (`Timeline|Timeline` :!via `PlayFromStart`)
    (:`Update`
      (bind _returnvalue_4 (* _dissolve (`self.DissolveDistance`)))
      (`MaterialInstanceDynamic.SetScalarParameterValue` _material "Dissolve Distance" _returnvalue_4)
      (`NiagaraComponent.SetVariableFloat` (`self.Niagara System`) "Dissolve Distance" _returnvalue_4)
      (`LightComponent.SetIntensity` (`self.PointLight`) (* _light_intensity 1.0)))
    (:`Finished`
      (`MaterialInstanceDynamic.SetScalarParameterValue` _material "Dissolve Distance" 0.0))))

(fn `UserConstructionScript`
  (bind (_min _max) (`StaticMeshComponent.GetLocalBounds` (`self.StaticMeshComp`)))
  (bind _returnvalue (`PrimitiveComponent.CreateDynamicMaterialInstance` (`self.StaticMeshComp`) 0 "/Game/HT/Resources/Meshes/BrokenCamera/M_Camera.M_Camera" "None"))
  (set `self.Material` _returnvalue)
  (set `self.DissolveDistance` (* (`KismetMathLibrary.VSize` (- _max _min)) 0.5)))